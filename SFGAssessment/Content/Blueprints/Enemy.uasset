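; Enemy Blueprint that takes damage from ammo and awards score for the current level when its health runs out.
; Each overlap with an Ammo actor, after the parent handler runs, subtracts one Health.
; At zero or below, it increments the current level's LevelScores entry in TheGameInstance.
; The enemy is not destroyed here, so further hits at zero or below score again.
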(event `self.ReceiveActorBeginOverlap`
  (params (OtherActor :type "Actor Object Reference"))
  (`parent.ReceiveActorBeginOverlap` OtherActor)
  (cast `/Game/Blueprints/Ammo` OtherActor)
  (bind _output_get (set `self.Health` (- (`self.Health`) 1)))
  (if (<= _output_get 0)
    (bind _asthe_game_instance (cast `/Game/Blueprints/TheGameInstance` (`GameplayStatics.GetGameInstance`)))
    (bind _levelscores (`/Game/Blueprints/TheGameInstance.LevelScores` _asthe_game_instance))
    (bind _returnvalue (- (`/Game/Blueprints/TheGameInstance.ThisLevel` _asthe_game_instance) 1))
    (`KismetArrayLibrary.Array_Set` _levelscores _returnvalue (+ (`|GetArrayItem` _levelscores _returnvalue) 1))))

(fn `UserConstructionScript`
  (`parent.UserConstructionScript`))