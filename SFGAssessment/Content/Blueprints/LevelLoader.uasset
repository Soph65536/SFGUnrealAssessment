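; LevelLoader is an actor that acts as a trigger cube for travelling to another level.
; Any overlap with the cube plays the EnterLevel sound, stores LevelToLoad in TheGameInstance as ThisLevel, then opens LevelMap by object reference.
; A disconnected switch on LevelToLoad would assign tutorial or numbered level icon materials to the cube, but it never runs.
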(event `self.ReceiveBeginPlay`
  (`parent.ReceiveBeginPlay`))

(event `self.Cube.OnComponentBeginOverlap`
  (params (OverlappedComponent :type "PrimitiveComponent Object Reference") (OtherActor :type "Actor Object Reference") (OtherComp :type "PrimitiveComponent Object Reference") (OtherBodyIndex :type Integer) (bFromSweep :type Boolean) (SweepResult :type "HitResult Structure (by ref)"))
  (`GameplayStatics.PlaySoundAtLocation` "/Game/Sounds/EnterLevel.EnterLevel" (`self.K2_GetActorLocation`) (struct) 1.0 1.0 0.0 null null null)
  (bind _asthe_game_instance (cast `/Game/Blueprints/TheGameInstance` (`GameplayStatics.GetGameInstance`)))
  (set `/Game/Blueprints/TheGameInstance.ThisLevel` (`self.LevelToLoad`) _asthe_game_instance)
  (`GameplayStatics.OpenLevelBySoftObjectPtr` "/Game/Maps/Levelmap.LevelMap"))

(event `self.ReceiveActorBeginOverlap`
  (params (OtherActor :type "Actor Object Reference"))
  (`parent.ReceiveActorBeginOverlap` OtherActor))

(fn `UserConstructionScript`
  (`parent.UserConstructionScript`))