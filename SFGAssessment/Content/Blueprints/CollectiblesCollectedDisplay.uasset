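; CollectiblesCollectedDisplay is an actor that shows how many collectibles have been collected.
; On BeginPlay it reads CollectiblesCollected from TheGameInstance and writes the number into its CollectiblesText component.
; The value is set only once at start, with no later refresh, and nothing is written if the game instance cast fails.
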(event `self.ReceiveBeginPlay`
  ;[1 1 1] show collectibles
  (`parent.ReceiveBeginPlay`)
  (bind _asthe_game_instance (cast `/Game/Blueprints/TheGameInstance` (`GameplayStatics.GetGameInstance`)))
  (`TextRenderComponent.K2_SetText` (`self.Collectibles Text`) (`KismetTextLibrary.Conv_IntToText` (`/Game/Blueprints/TheGameInstance.CollectiblesCollected` _asthe_game_instance))))

(fn `UserConstructionScript`
  (`parent.UserConstructionScript`))