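; LevelPlayerPawn is a player pawn that handles mouse look and tilts the view with horizontal input.
; Mouse axes add controller pitch and yaw, then share the horizontal axis's rotation update, which clamps both to MaxRotationAngle.
; That update also eases roll toward the horizontal input scaled by MaxRollAngle, using FInterpTo, and writes the result to the control rotation.
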(event `InputAxis|HorizontalMovement`
  (params (AxisValue :type "Float (single-precision)"))
  (bind (_returnvalue_roll _returnvalue_pitch _returnvalue_yaw) (`KismetMathLibrary.BreakRotator` (`self.GetControlRotation`)))
  (bind _returnvalue_roll_2 (`KismetMathLibrary.BreakRotator` (`self.GetControlRotation`)))
  (bind _maxrotationangle (`self.MaxRotationAngle`))
  (bind _maxrollangle (`self.MaxRollAngle`))
  (bind _returnvalue (* -1 _maxrotationangle))
  ;[1 1 1] Rotate camera with horizontal input and interpolate
  ;[1 1 1] Set Rotation
  (`Controller.SetControlRotation` (`GameplayStatics.GetPlayerController` 0) (`KismetMathLibrary.MakeRotator` (`KismetMathLibrary.FInterpTo` _returnvalue_roll_2 (`KismetMathLibrary.ClampAngle` (* AxisValue _maxrollangle) (* -1 _maxrollangle) _maxrollangle) (`GameplayStatics.GetWorldDeltaSeconds`) 0.5) (`KismetMathLibrary.ClampAngle` _returnvalue_pitch _returnvalue _maxrotationangle) (`KismetMathLibrary.ClampAngle` _returnvalue_yaw _returnvalue _maxrotationangle)) :!label _label))

(event `InputAxis|MouseLookVertical`
  (params (AxisValue :type "Float (single-precision)"))
  ;[1 1 1] Camera Rotation with clamp
  (`self.AddControllerPitchInput` AxisValue)
  (goto _label))

(event `InputAxis|MouseLookHorizontal`
  (params (AxisValue :type "Float (single-precision)"))
  ;[1 1 1] Camera Rotation with clamp
  (`self.AddControllerYawInput` AxisValue)
  (goto _label))

(fn `UserConstructionScript`)