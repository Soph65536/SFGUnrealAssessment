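; Collectible actor that triggers once when an Ammo actor overlaps it, damaging every enemy in the level.
; It plays its audio and particle effect, then takes one Health from each Enemy found with GetAllActorsOfClass.
; It then increments CollectiblesCollected on TheGameInstance and destroys itself after a short delay.
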(event `self.ReceiveActorBeginOverlap`
  (params (OtherActor :type "Actor Object Reference"))
  ;[1 1 1] play effects and hit all enemies
  (`parent.ReceiveActorBeginOverlap` OtherActor)
  (cast `/Game/Blueprints/Ammo` OtherActor)
  (`/Engine/EditorBlueprintResources/StandardMacros.DoOnce` false
    (:`Completed`
      (`AudioComponent.Play` (`self.Audio`) 0.0)
      (`ActorComponent.Activate` (`self.ParticleSystem`) false)
      (bind _outactors (`GameplayStatics.GetAllActorsOfClass` "/Game/Blueprints/Enemy.Enemy_C"))
      (for _array_element _outactors
        (bind _result (`/Engine/EditorBlueprintResources/StandardMacros.DecrementInt` (`/Game/Blueprints/Enemy.Health` _array_element))
          (:`  `
            (set `/Game/Blueprints/Enemy.Health` _result _array_element))))
      ;[1 1 1] increment collectibles and destroy this
      (bind _asthe_game_instance (cast `/Game/Blueprints/TheGameInstance` (`GameplayStatics.GetGameInstance`)))
      (bind _result_2 (`/Engine/EditorBlueprintResources/StandardMacros.IncrementInt` (`/Game/Blueprints/TheGameInstance.CollectiblesCollected` _asthe_game_instance))
        (:`  `
          (set `/Game/Blueprints/TheGameInstance.CollectiblesCollected` _result_2 _asthe_game_instance)
          (`KismetSystemLibrary.Delay` 2.0)
          (`self.K2_DestroyActor`))))))

(fn `UserConstructionScript`
  (`parent.UserConstructionScript`))