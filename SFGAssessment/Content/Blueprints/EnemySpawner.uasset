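; Enemy spawner actor that repeatedly spawns an Enemy at its own transform, tuned to the current level.
; BeginPlay reads ThisLevel from TheGameInstance and sets SpawnDelay for levels 1 to 6.
; Tick runs through a Delay node, which acts as a repeating spawn timer, then sets each new enemy's Health from the same level number.
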(event `self.ReceiveTick`
  (params (DeltaSeconds :type "Float (single-precision)"))
  ;[1 1 1] wait for spawndelay seconds then spawn enemy
  (`KismetSystemLibrary.Delay` (`self.SpawnDelay`))
  (bind _returnvalue (`|SpawnActorFromClass` "/Game/Blueprints/Enemy.Enemy_C" (`self.GetTransform`) "Undefined" "OverrideRootScale" null null))
  ;[1 1 1] set enemy health based on thislevel
  (switch `int` (`/Game/Blueprints/TheGameInstance.ThisLevel` (stale `self.ReceiveBeginPlay` _asthe_game_instance))
    (:`1`
      (set `/Game/Blueprints/Enemy.Health` 1 _returnvalue))
    (:`2`
      (set `/Game/Blueprints/Enemy.Health` 2 _returnvalue))
    (:`3`
      (set `/Game/Blueprints/Enemy.Health` 3 _returnvalue))
    (:`4`
      (set `/Game/Blueprints/Enemy.Health` 4 _returnvalue))
    (:`5`
      (set `/Game/Blueprints/Enemy.Health` 5 _returnvalue))
    (:`6`
      (set `/Game/Blueprints/Enemy.Health` 10 _returnvalue))))

(event `self.ReceiveBeginPlay`
  ;[1 1 1] set spawndelay based on thislevel
  (bind _asthe_game_instance (cast `/Game/Blueprints/TheGameInstance` (`GameplayStatics.GetGameInstance`)))
  (switch `int` (`/Game/Blueprints/TheGameInstance.ThisLevel` _asthe_game_instance)
    (:`1`
      (set `self.SpawnDelay` 5.0))
    (:`2`
      (set `self.SpawnDelay` 4.0))
    (:`3`
      (set `self.SpawnDelay` 5.0))
    (:`4`
      (set `self.SpawnDelay` 6.0))
    (:`5`
      (set `self.SpawnDelay` 8.0))
    (:`6`
      (set `self.SpawnDelay` 10.0))))

(fn `UserConstructionScript`)